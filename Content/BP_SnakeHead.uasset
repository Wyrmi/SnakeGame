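; Player-controlled head of a Snake game that moves each tick, spawns tail segments and tracks score.
; Directional input sets the move direction, checked against the last actual movement to block reversals.
; Tick steps the head by its mesh width, shifts each tail into its predecessor's old position, then wraps the head at the border.
; AddTail grows the body, while AddScore updates the score widget created at BeginPlay.
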(event Custom|AddTail
  (bind _returnvalue (Game|SpawnActorfromClass "/Game/Tail.Tail_C" (Math|Transform|MakeTransform (- (Transformation|GetActorLocation) (* (Variables|Default|GetMoveDir) (Variables|Default|GetStepSize))) "0, 0, 0" "1,1,1") "Undefined" 0 0))
  (Utilities|Array|Add (Variables|Default|GetTails) _returnvalue))

(event Custom|AddScore
  (bind _result (Math|Integer|IncrementInt (Variables|Default|GetScore))
    (:%20%20
      (Default|SetScore (Variables|Default|GetMainUI) _result))))

(event EventBeginPlay
  (bind _snakehead (Variables|Default|GetSnakeHead))
  (bind _staticmesh (Variables|/Script/Engine.StaticMeshComponent|GetStaticMesh _snakehead))
  (bind _returnvalue (StaticMesh|GetBoundingBox _staticmesh))
  (Variables|Default|SetStepSize (- (.x (.max _returnvalue)) (.x (.min _returnvalue))))
  (bind _returnvalue_2 (UserInterface|CreateWidget "/Game/Score.Score_C" (Game|GetPlayerController 0)))
  (bind _output_get (Variables|Default|SetMainUI _returnvalue_2))
  (UserInterface|Viewport|AddtoViewport _output_get 0))

(event Collision|EventActorBeginOverlap
  (params (OtherActor :type Actor%20Object%20Reference)))

(event EventTick
  (params (DeltaSeconds :type Float%20%28single-precision%29))
  (bind _returnvalue (Transformation|GetActorLocation))
  (bind _border (Variables|Default|GetBorder))
  (bind _output_get (Variables|Default|SetPreMoveLocation (Transformation|GetActorLocation)))
  (Transformation|AddActorWorldOffset (* (Variables|Default|GetMoveDir) (Variables|Default|GetStepSize)))
  (Variables|Default|SetCurrentDir (- (Transformation|GetActorLocation) _output_get))
  (for _array_element (Variables|Default|GetTails)
    (bind _output_get_2 (Variables|Default|SetCurrentTailLocation (Transformation|GetActorLocation _array_element)))
    (Transformation|SetActorLocation _array_element (Variables|Default|GetPreMoveLocation) false false)
    (Variables|Default|SetPreMoveLocation _output_get_2))
  (if (> (Math|Float|Absolute(Float) (.x _returnvalue)) _border)
    (Transformation|SetActorLocation (Math|Vector|MakeVector (* -1 (.x _returnvalue)) (.y _returnvalue) (.z _returnvalue)) false true))
  (if (> (Math|Float|Absolute(Float) (.y _returnvalue)) _border)
    (Transformation|SetActorLocation (Math|Vector|MakeVector (.x _returnvalue) (* -1 (.y _returnvalue)) (.z _returnvalue)) false true)))

(event Input|ActionEvents|InputActionUp
  (params (Key :type Key%20Structure :default "None"))
  (:Pressed
    (if (== (.x (Variables|Default|GetCurrentDir)) 0.0)
      (Variables|Default|SetMoveDir "1.000000, 0, 0"))))

(event Input|ActionEvents|InputActionDown
  (params (Key :type Key%20Structure :default "None"))
  (:Pressed
    (if (== (.x (Variables|Default|GetCurrentDir)) 0.0)
      (Variables|Default|SetMoveDir "-1.000000, 0, 0"))))

(event Input|ActionEvents|InputActionLeft
  (params (Key :type Key%20Structure :default "None"))
  (:Pressed
    (if (== (.y (Variables|Default|GetCurrentDir)) 0.0)
      (Variables|Default|SetMoveDir "0.000000,-1.000000, 0"))))

(event Input|ActionEvents|InputActionRight
  (params (Key :type Key%20Structure :default "None"))
  (:Pressed
    (if (== (.y (Variables|Default|GetCurrentDir)) 0.0)
      (Variables|Default|SetMoveDir "0.000000,1.000000, 0"))))

(fn ConstructionScript)